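; Standing torch actor that lights up at night and shuts off during the day.
; Day and Night events toggle its fire particles, point light, audio and trigger sphere.
; Overlapping the sphere, sized on BeginPlay, fades the fire sound in and out.
; While night, a delayed Tick randomizes light intensity for flicker, but also sets attenuation radius to zero, leaving the random range unused.
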(event OnComponentBeginOverlap(Sphere)
  (params (OverlappedComponent :type Primitive%20Component%20Object%20Reference) (OtherActor :type Actor%20Object%20Reference) (OtherComp :type Primitive%20Component%20Object%20Reference) (OtherBodyIndex :type Integer) (bFromSweep :type Boolean) (SweepResult :type Hit%20Result%20Structure%20%28by%20ref%29))
  ;[1 1 1] sound fade in and out
  (Audio|Components|Audio|FadeIn (Variables|Default|GetAudio) (Variables|Default|Getaudiofade) (Variables|Default|Getfirevolume) 0.0 :!class /Script/Engine.AudioComponent))

(event OnComponentEndOverlap(Sphere)
  (params (OverlappedComponent :type Primitive%20Component%20Object%20Reference) (OtherActor :type Actor%20Object%20Reference) (OtherComp :type Primitive%20Component%20Object%20Reference) (OtherBodyIndex :type Integer))
  ;[1 1 1] sound fade in and out
  (Audio|Components|Audio|FadeOut (Variables|Default|GetAudio) (Variables|Default|Getaudiofade) 0.0 :!class /Script/Engine.AudioComponent))

(event EventBeginPlay
  (bind _sphere (Variables|Default|GetSphere))
  ;[1 1 1] begin setup
  (Components|Sphere|SetSphereRadius _sphere (Variables|Default|GetsoundRadius) true)
  (Transformation|SetWorldScale3D _sphere (Variables|Default|GetSoundScale)))

(event EventDay
  ;[1 1 1] set on / off
  (Components|Activation|SetActive (Variables|Default|GetAudio) false false)
  (Components|Activation|SetActive (Variables|Default|GetSphere) false false)
  (Components|Activation|SetActive (Variables|Default|GetParticleSystem) false false)
  (Rendering|SetVisibility (Variables|Default|GetPointLight) false false)
  (Variables|Default|SetNightTrue false))

(event EventNight
  ;[1 1 1] set on / off
  (Components|Activation|SetActive (Variables|Default|GetAudio) true false)
  (Components|Activation|SetActive (Variables|Default|GetSphere) true false)
  (Components|Activation|SetActive (Variables|Default|GetParticleSystem) true false)
  (Rendering|SetVisibility (Variables|Default|GetPointLight) true false)
  (Variables|Default|SetNightTrue true))

(event EventTick
  (params (DeltaSeconds :type Float%20%28single-precision%29))
  (bind _pointlight (Variables|Default|GetPointLight))
  ;[1 1 1] light variability
  (Utilities|FlowControl|Delay 0.2)
  (if (Variables|Default|GetNightTrue)
    (Rendering|Components|Light|SetIntensity _pointlight (Math|Random|RandomFloatinRange (Variables|Default|GetMinIntensity) (Variables|Default|GetMaxIntensity)))
    (Rendering|Lighting|SetAttenuationRadius _pointlight 0.0)))

(fn ConstructionScript)