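; BP_Torch is a torch actor with fire particles, point light and audio that Day and Night events switch off and on.
; A sphere, sized at BeginPlay, fades the fire sound in on any overlap and cuts it on exit.
; At night, a Delay on Tick throttles random intensity flicker.
; The same step sets attenuation radius to zero, leaving the random-range node unused.
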(event OnComponentBeginOverlap(Sphere)
  (params (OverlappedComponent :type Primitive%20Component%20Object%20Reference) (OtherActor :type Actor%20Object%20Reference) (OtherComp :type Primitive%20Component%20Object%20Reference) (OtherBodyIndex :type Integer) (bFromSweep :type Boolean) (SweepResult :type Hit%20Result%20Structure%20%28by%20ref%29))
  ;[1 1 1] sound fade in and out
  (Audio|Components|Audio|FadeIn (Variables|Default|GetAudio) (Variables|Sound|GetAudioFade) (Variables|Sound|GetfireVolume) 0.0 :!class /Script/Engine.AudioComponent))

(event OnComponentEndOverlap(Sphere)
  (params (OverlappedComponent :type Primitive%20Component%20Object%20Reference) (OtherActor :type Actor%20Object%20Reference) (OtherComp :type Primitive%20Component%20Object%20Reference) (OtherBodyIndex :type Integer))
  ;[1 1 1] sound fade in and out
  (Audio|Components|Audio|FadeOut (Variables|Default|GetAudio) 0.0 0.0 :!class /Script/Engine.AudioComponent))

(event EventBeginPlay
  (bind _sphere (Variables|Default|GetSphere))
  ;[1 1 1] begin setup
  (Components|Sphere|SetSphereRadius _sphere (Variables|Sound|GetsoundRadius) true)
  (Transformation|SetWorldScale3D _sphere (Variables|Sound|GetSound%20Scale)))

(event EventDay
  ;[1 1 1] set on / off
  (Components|Activation|SetActive (Variables|Default|GetAudio) false false)
  (Components|Activation|SetActive (Variables|Default|GetSphere) false false)
  (Components|Activation|SetActive (Variables|Default|GetP_TorchFire) false false)
  (Rendering|SetVisibility (Variables|Default|GetPointLight) false false)
  (Variables|Default|SetnightTrue false))

(event EventNight
  (bind _pointlight (Variables|Default|GetPointLight))
  ;[1 1 1] set on / off
  (Components|Activation|SetActive (Variables|Default|GetAudio) true false)
  (Components|Activation|SetActive (Variables|Default|GetSphere) true false)
  (Components|Activation|SetActive _pointlight true false)
  (Rendering|SetVisibility _pointlight true false)
  (Variables|Default|SetnightTrue true))

(event EventTick
  (params (DeltaSeconds :type Float%20%28single-precision%29))
  (bind _pointlight (Variables|Default|GetPointLight))
  ;[1 1 1] light variability
  (Utilities|FlowControl|Delay 0.2)
  (if (Variables|Default|GetnightTrue)
    (Rendering|Components|Light|SetIntensity _pointlight (Math|Random|RandomFloatinRange (Variables|Default|GetMinintensity) (Variables|Default|Getmaxintensity)))
    (Rendering|Lighting|SetAttenuationRadius _pointlight 0.0)))

(fn ConstructionScript)