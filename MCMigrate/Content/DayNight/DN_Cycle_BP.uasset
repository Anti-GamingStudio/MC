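; Day/night cycle Blueprint that rotates sun and moon lights and notifies DayNightInterface actors of day or night.
; Tick advances Hour from the configured day length, derives SunAngle, and updates the sky and opposed lights after a Delay.
; An angle range check calls day or night events every tick, rebroadcasting messages and resetting Hour when day returns.
; These events drive timelines for post-process, clouds, moon intensity and visibility, plus skylight color interpolation and shadow switching.
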(event Custom|dayEvent
  (bind _moon_ref (Variables|LevelRef|Getmoon_ref))
  (bind _sun (Variables|LevelRef|GetSun))
  (bind _skylight (Variables|LevelRef|GetSkyLight))
  (bind _lightcomponent (Variables|/Script/Engine.Light|GetLightComponent _sun))
  (bind _lightcomponent_2 (Variables|/Script/Engine.SkyLight|GetLightComponent _skylight))
  (bind _lightcomponent_3 (Variables|/Script/Engine.Light|GetLightComponent _moon_ref))
  ;[1 1 1] Effects
  ;;[1 1 1] D / N calls
  (Utilities|FlowControl|Sequence
    (:then_0
      (bind _outactors (Actor|GetAllActorswithInterface "/Game/DayNightInterface.DayNightInterface_C"))
      (for _array_element _outactors
        (Class|DayNightInterface|Day(Message) _array_element)))
    (:then_1
      ;;[1 1 1] PostProcess ON / OFF
      (bind (_direction _newtrack_0 _newtrack_1) (Timeline|blend%20weight Reverse)
        (:Update
          (Variables|/Script/Engine.PostProcessComponent|SetBlendWeight (Variables|Default|GetPostProcess) _newtrack_0)
          (Variables|/Script/Engine.PostProcessComponent|SetBlendWeight (Variables|Default|Geteyyyy) _newtrack_1))))
    (:then_2
      ;;[1 1 1] SKY LIGHT
      (Rendering|Components|Light|SetLightColor _lightcomponent_2 (Class|KismetMathLibrary|CInterpto (Rendering|Components|Light|GetLightColor _lightcomponent_2) (Variables|Settings|GetColor%20Of%20Day%20Light) (Variables|Default|GetDeltaTime) (Variables|Settings|GetLightingChangeSpeed)))
      (Rendering|Components|Light|SetIntensity _lightcomponent_2 3.0))
    (:then_3
      ;;[1 1 1] sets cloud opacity
      (bind _newtrack_0_2 (Timeline|Timeline_0 Play)
        (:Update
          (Variables|/Engine/EngineSky/BP_Sky_Sphere.BP_Sky_Sphere_C|SetCloud%20opacity (Variables|LevelRef|GetSky) _newtrack_0_2))))
    (:then_4
      ;[1 1 1] controls lighjting
      (Rendering|Components|Light|SetCastShadows _lightcomponent true)
      (Rendering|Components|Light|SetCastShadows _lightcomponent_3 false)
      (Rendering|SetVisibility _lightcomponent true true)
      (bind (_direction_2 _newtrack_1_2 _newtrack_2) (Timeline|Timeline_1 Play)
        (:Update
          ;;[1 1 1] sun
          (Utilities|FlowControl|Sequence
            (:then_0
              (Rendering|Components|Light|SetIntensity _lightcomponent_3 _newtrack_1_2))
            (:then_1
              ;;[1 1 1] moon
              (Rendering|Components|Light|SetIntensity _lightcomponent_3 _newtrack_2))))
        (:Finished
          (if (Variables|Default|GetDay)
            (Rendering|SetVisibility _lightcomponent_3 false true)
            (bind _newtrack_1_3 (Timeline|eyy Play)
              (:Update
                (Variables|/Engine/EngineSky/BP_Sky_Sphere.BP_Sky_Sphere_C|SetSun%20brightness (Variables|LevelRef|GetSky) _newtrack_1_3)))
            (else
              (Rendering|SetVisibility _lightcomponent false true)
              (Timeline|eyy Reverse))))))))

(event Custom|nightevent
  (bind _moon_ref (Variables|LevelRef|Getmoon_ref))
  (bind _sun (Variables|LevelRef|GetSun))
  (bind _skylight (Variables|LevelRef|GetSkyLight))
  (bind _lightcomponent (Variables|/Script/Engine.Light|GetLightComponent _sun))
  (bind _lightcomponent_2 (Variables|/Script/Engine.SkyLight|GetLightComponent _skylight))
  (bind _lightcomponent_3 (Variables|/Script/Engine.Light|GetLightComponent _moon_ref))
  ;[1 1 1] Effects
  ;;[1 1 1] D / N calls
  (Utilities|FlowControl|Sequence
    (:then_0
      ;;[1 1 1] PostProcess ON / OFF
      (bind (_direction _newtrack_0 _newtrack_1) (Timeline|blend%20weight Play)
        (:Update
          (Variables|/Script/Engine.PostProcessComponent|SetBlendWeight (Variables|Default|GetPostProcess) _newtrack_0)
          (Variables|/Script/Engine.PostProcessComponent|SetBlendWeight (Variables|Default|Geteyyyy) _newtrack_1))))
    (:then_1
      ;;[1 1 1] SKY LIGHT
      (Rendering|Components|Light|SetLightColor _lightcomponent_2 (Class|KismetMathLibrary|CInterpto (Rendering|Components|Light|GetLightColor _lightcomponent_2) (Variables|Settings|GetColorOfNightLight) (Variables|Default|GetDeltaTime) (Variables|Settings|GetLightingChangeSpeed)))
      (Rendering|Components|Light|SetIntensity _lightcomponent_2 3.0))
    (:then_2
      ;;[1 1 1] sets cloud opacity
      (bind _newtrack_0_2 (Timeline|Timeline_0 Reverse)
        (:Update
          (Variables|/Engine/EngineSky/BP_Sky_Sphere.BP_Sky_Sphere_C|SetCloud%20opacity (Variables|LevelRef|GetSky) _newtrack_0_2))))
    (:then_3
      ;[1 1 1] controls lighjting
      (Rendering|Components|Light|SetCastShadows _lightcomponent false)
      (Rendering|Components|Light|SetCastShadows _lightcomponent_3 true)
      (Rendering|SetVisibility _lightcomponent_3 true true)
      (bind (_direction_2 _newtrack_1_2 _newtrack_2) (Timeline|Timeline_1 Reverse)
        (:Update
          ;;[1 1 1] sun
          (Utilities|FlowControl|Sequence
            (:then_0
              (Rendering|Components|Light|SetIntensity _lightcomponent_3 _newtrack_1_2))
            (:then_1
              ;;[1 1 1] moon
              (Rendering|Components|Light|SetIntensity _lightcomponent_3 _newtrack_2))))
        (:Finished
          (if (Variables|Default|GetDay)
            (Rendering|SetVisibility _lightcomponent_3 false true)
            (bind _newtrack_1_3 (Timeline|eyy Play)
              (:Update
                (Variables|/Engine/EngineSky/BP_Sky_Sphere.BP_Sky_Sphere_C|SetSun%20brightness (Variables|LevelRef|GetSky) _newtrack_1_3)))
            (else
              (Rendering|SetVisibility _lightcomponent false true)
              (Timeline|eyy Reverse))))))
    (:then_4
      (bind _outactors (Actor|GetAllActorswithInterface "/Game/DayNightInterface.DayNightInterface_C"))
      (for _array_element _outactors
        (Class|DayNightInterface|Night(Message) _array_element)))))

(event EventBeginPlay
  ;[1 1 1] sets default parameters that determine later calculation
  (bind _output_get (Variables|Default|SetOneDay (* (Variables|Settings|GetDayLengthInMin) 6e+01)))
  (Variables|Default|SetOneHour (/ _output_get 24.0))
  (Default|UpdateSunDirection (Variables|LevelRef|GetSky))
  (if (Math|Float|InRange(Float) (Variables|Default|GetSunAngle) (Variables|Settings|GetDayStart%28Light%20Rotation%29) (Variables|Settings|GetDayEnd%28light%20Rotation%29))
    (Variables|Default|SetDay true)
    (bind _outactors (Actor|GetAllActorswithInterface "/Game/DayNightInterface.DayNightInterface_C"))
    (for _array_element _outactors
      (Class|DayNightInterface|Day(Message) _array_element))
    (else
      (Variables|Default|SetDay false)
      (bind _outactors_2 (Actor|GetAllActorswithInterface "/Game/DayNightInterface.DayNightInterface_C"))
      (for _array_element_2 _outactors_2
        (Class|DayNightInterface|Night(Message) _array_element_2)))))

(event EventTick
  (params (DeltaSeconds :type Float%20%28single-precision%29))
  ;[1 1 1] calculates time and sets rotation accordingly
  (Utilities|FlowControl|Sequence
    (:then_0
      (if (Variables|Settings|GetDayNightCycle%20ON)
        (Utilities|FlowControl|Sequence
          (:then_0
            (bind _output_get (Variables|Settings|SetHour (+ (Variables|Settings|GetHour) (/ DeltaSeconds (Variables|Default|GetOneHour)))))
            (bind _output_get_2 (Variables|Default|SetSunAngle (* _output_get 15.0)))
            (Utilities|FlowControl|Delay (Variables|Settings|GetUpdateRate))
            (Transformation|SetActorRotation (Variables|LevelRef|GetSun) (Math|Rotator|MakeRotator 0.0 _output_get_2 23.5))
            (Default|UpdateSunDirection (Variables|LevelRef|GetSky))
            (Transformation|SetWorldRotation (Variables|Default|GetmoonDistance) (Math|Rotator|MakeRotator 0.0 (+ _output_get_2 1.8e+02) 23.5) false false)
            (Transformation|SetActorRotation (Variables|LevelRef|Getmoon_ref) (Math|Rotator|MakeRotator 0.0 (+ _output_get_2 1.8e+02) 23.5)))
          (:then_1
            ;[1 1 1] Sets Day/Night Depending on the rotation of the Directrional light
            (if (Math|Float|InRange(Float) (Variables|Default|GetSunAngle) (Variables|Settings|GetDayStart%28Light%20Rotation%29) (Variables|Settings|GetDayEnd%28light%20Rotation%29))
              (Variables|Default|SetDay true)
              (CallFunction|DayEvent)
              (goto _label Reset)
              (else
                (Variables|Default|SetDay false)
                (CallFunction|Nightevent)
                (Utilities|FlowControl|DoOnce true :!label _label
                  (:Completed
                    (Variables|Settings|SetHour 0.0)))))))))
    (:then_1
      (Variables|Default|SetDeltaTime DeltaSeconds))))

(fn ConstructionScript)